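; AI controller for BP_NPC that runs the BT_NPC behavior tree and tracks whether the NPC acts as a guard or a player chaser.
; Perception of the player sets CanSeePlayer on the blackboard and, outside guard mode, switches the state between Chase and Random.
; Every Tick copies the pawn's guard flags to the blackboard, picks Protect or Patrol for guards, and updates the NPC's colored task text to match the state.
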(event OnTargetPerceptionUpdated(AIPerception)
  (params (Actor :type Actor%20Object%20Reference) (Stimulus :type AI%20Stimulus%20Structure))
  (bind _bsuccessfullysensed (Utilities|Struct|BreakAIStimulus Stimulus))
  ;[1 0.3495 0.02461] Update Blackboard Bool based on if AI can see player
  (Utilities|Casting|CastToThirdPersonCharacter Actor)
  (AI|Components|Blackboard|SetValueasBool (AI|GetBlackboard 0) (Utilities|Name|MakeLiteralName "CanSeePlayer") _bsuccessfullysensed)
  (bind _asbp_npc (Utilities|Casting|CastToBP_NPC (Pawn|GetControlledPawn)))
  (if (not (Variables|/Game/MyContent/BP/NPC/BP_NPC.BP_NPC_C|GetGuardMode _asbp_npc))
    (if _bsuccessfullysensed
      (Variables|Default|SetState "Chase")
      (else
        (Variables|Default|SetState "Random")))))

(event EventBeginPlay
  ;[0.165 1 0.2109] On play Run the NPC's Behavior Tree
  (AI|RunBehaviorTree "/Game/MyContent/BP/NPC/BT_NPC.BT_NPC"))

(event EventTick
  (params (DeltaSeconds :type Float%20%28single-precision%29))
  (Utilities|FlowControl|Sequence
    (:then_0
      ;[0.1124 0.2001 1] Friendly vs Enemy AI Checks
      (bind _asbp_npc (Utilities|Casting|CastToBP_NPC (Pawn|GetControlledPawn)))
      (AI|Components|Blackboard|SetValueasBool (AI|GetBlackboard 0) (Utilities|Name|MakeLiteralName "GuardMode") (Variables|/Game/MyContent/BP/NPC/BP_NPC.BP_NPC_C|GetGuardMode _asbp_npc))
      ;[0.7563 1 0.02974] Init Friendly Text
      (if (Variables|/Game/MyContent/BP/NPC/BP_NPC.BP_NPC_C|GetGuardMode _asbp_npc)
        (if (Variables|/Game/MyContent/BP/NPC/BP_NPC.BP_NPC_C|GetGuardFollow _asbp_npc)
          (Variables|Default|SetState "Protect")
          ;[0 1 0.02487] Set Guard AI Blackboard Varribles
          (AI|Components|Blackboard|SetValueasBool (AI|GetBlackboard 0) (Utilities|Name|MakeLiteralName "GuardFollow") (Variables|/Game/MyContent/BP/NPC/BP_NPC.BP_NPC_C|GetGuardFollow _asbp_npc))
          (else
            (Variables|Default|SetState "Patrol")
            (AI|Components|Blackboard|SetValueasBool (AI|GetBlackboard 0) (Utilities|Name|MakeLiteralName "GuardMode") (Variables|/Game/MyContent/BP/NPC/BP_NPC.BP_NPC_C|GetGuardMode _asbp_npc))))))
    (:then_1
      ;[0.2116 0.06317 0.2135] Setting text based of state
      (bind _asbp_npc_2 (Utilities|Casting|CastToBP_NPC (Pawn|GetControlledPawn)))
      (switch string (Variables|Default|GetState)
        (:Protect
          ;;[0.1468 1 0.02884] Update NPC: < Protect Player >
          (Default|UpdateTask _asbp_npc_2 "< Protect Player >" 2))
        (:Chase
          ;;[1 0 0.02604] Update NPC: Follow Player
          (Default|UpdateTask _asbp_npc_2 "< Following Player >" 3))
        (:Patrol
          ;;[0 0.2829 1] Update NPC: Patrol
          (Default|UpdateTask _asbp_npc_2 "< Guard: Patroling  >" 4))
        (:Random
          ;;[1 0.9448 0] Update NPC: Random Locaton
          (Default|UpdateTask _asbp_npc_2 "< Moving to Random Location >" 5))))))

(fn ConstructionScript)